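; Greenskin NPC character that caches its AI controller and NPC movement component, and handles enemy detection and combat animation.
; About once a second, Tick passes NPCs overlapping its collider to the movement component's FilterEnemies.
; Move-state events switch the Ork anim blueprint from attacking to walking.
; Attack events play an indexed montage and re-enable CanAttack when it completes.
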(event `self.ReceiveBeginPlay`
  (bind _asnpc_controller (cast `NPC_Controller` (`AIBlueprintHelperLibrary.GetAIController` self))
    (:`then`
      (set `self.npcController` _asnpc_controller))
    (:`CastFailed`
      (`KismetSystemLibrary.PrintString` "Greenskin controller cast failed"))))

(event `self.ReceiveTick`
  (params (DeltaSeconds :type "Float (single-precision)"))
  (bind _overlapcollider (`self.OverlapCollider`))
  (bind _output_get (set `self.timer` (+ (stale _output_get) DeltaSeconds)))
  (if (> _output_get 1.0)
    (`PrimitiveComponent.IgnoreActorWhenMoving` _overlapcollider self true)
    (`PrimitiveComponent.IgnoreActorWhenMoving` (`self.CapsuleComponent`) self true)
    (bind _asnpcmovement_component (cast `NPCMovementComponent` (`self.CharacterMovement`)))
    (`NPCMovementComponent.FilterEnemies` _asnpcmovement_component (`PrimitiveComponent.GetOverlappingActors` _overlapcollider "/Script/Warhammer.NPC") (`self.npc`))
    (set `self.timer` 0.0)))

(event `self.inMoveState`
  (bind _asork_anim_bp (cast `/Game/Warhammer/Assets/Animations/Ork/Ork_Anim_BP` (`SkeletalMeshComponent.GetAnimInstance` (`self.Mesh`))))
  (set `/Game/Warhammer/Assets/Animations/Ork/Ork_Anim_BP.isAttacking` false _asork_anim_bp)
  (set `/Game/Warhammer/Assets/Animations/Ork/Ork_Anim_BP.isWalking` true _asork_anim_bp))

(event `self.PlayAttackAnimation`
  (params (i :type Integer))
  (`|PlayMontage` (`self.Mesh`) (`|GetArrayItem` (`self.attackAnims`) i)
    (:`OnCompleted`
      (set `self.canAttack` true))))

(fn `UserConstructionScript`
  (set `self.npc` self)
  (bind _asnpcmovement_component (cast `NPCMovementComponent` (`self.CharacterMovement`)))
  (set `self.movementComponent` _asnpcmovement_component))