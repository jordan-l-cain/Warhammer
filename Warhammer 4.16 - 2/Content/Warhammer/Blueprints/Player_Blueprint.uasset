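; Player Blueprint for the Warhammer game, a first-person-style controlled character with movement, mouse-look and an early selection interaction.
; Axis inputs move the player along the control rotation's yaw and feed controller yaw and pitch for looking.
; Interact fires a debug-drawn visibility line trace from the camera and prints the name of any TestAI hit.
; PlayerAttack is an empty stub.
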(event `InputAxis|Forward-Reverse`
  (params (AxisValue :type "Float (single-precision)"))
  ;[1 1 1] Movement Inputs for Forward/Backward and Left/Right
  (`self.AddMovementInput` (`KismetMathLibrary.GetForwardVector` (`KismetMathLibrary.MakeRotator` 0.0 0.0 (.yaw (`self.GetControlRotation`)))) AxisValue))

(event `InputAction|Interact`
  (params (Key :type "Key Structure" :default "AnyKey"))
  (bind _camera (`self.Camera`))
  (bind _returnvalue (`SceneComponent.K2_GetComponentLocation` _camera))
  ;[1 1 1] Will Handle Selection interaction/Add Interaction Interface
  (:`Pressed`
    (bind (_outhit _returnvalue_2) (`KismetSystemLibrary.LineTraceSingle` :`Start` _returnvalue :`End` (+ (* (`SceneComponent.GetForwardVector` _camera) 5000.0) _returnvalue) :`TraceChannel` "TraceTypeQuery1" :`DrawDebugType` "ForDuration"))
    (if _returnvalue_2
      (bind _astest_ai (cast `/Game/Warhammer/Blueprints/TestAI` (`.HitActor` (`GameplayStatics.BreakHitResult` _outhit))))
      (`KismetSystemLibrary.PrintString` (`KismetSystemLibrary.GetDisplayName` _astest_ai)))))

(event `InputAxis|Left-Right`
  (params (AxisValue :type "Float (single-precision)"))
  ;[1 1 1] Movement Inputs for Forward/Backward and Left/Right
  (`self.AddMovementInput` (`KismetMathLibrary.GetRightVector` (`KismetMathLibrary.MakeRotator` 0.0 0.0 (.yaw (`self.GetControlRotation`)))) AxisValue))

(event `InputAxis|Turn`
  (params (AxisValue :type "Float (single-precision)"))
  ;[1 1 1] Look Controls
  (`self.AddControllerYawInput` AxisValue))

(event `InputAxis|LookUp`
  (params (AxisValue :type "Float (single-precision)"))
  ;[1 1 1] Look Controls
  (`self.AddControllerPitchInput` AxisValue))

(fn `PlayerAttack`)

(fn `UserConstructionScript`)