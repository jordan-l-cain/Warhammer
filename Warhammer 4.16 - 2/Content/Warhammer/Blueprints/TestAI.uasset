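; TestAI is a prototype enemy character meant to patrol tagged points and move toward the player on sight, but its event and function entry points are unwired.
; The disconnected logic gathers PatrolPoint actors, cycles through them with AIMoveTo and pauses on a timer at each.
; Disconnected sight logic chases Player_Blueprint once through PawnSensing, halting within a path-length threshold.
; Only UnPauseAI, which clears the moving flag, has a connected body.
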(event `self.PawnSensing.OnSeePawn`
  (params (Pawn :type "Pawn Object Reference"))
  ;[1 1 1] How AI will handle seeing player
)

(event `self.ReceiveBeginPlay`
  ;[1 1 1] Creating Array for Patrol Points
)

(event `self.ReceiveTick`
  (params (DeltaSeconds :type "Float (single-precision)"))
  ;[1 1 1] Patrolling
)

(fn `NextDestination`)

(fn `UnPauseAI`
  (set `self.IsMoving` false)
  (`KismetSystemLibrary.PrintString` "Unpaused"))

(fn `UserConstructionScript`)