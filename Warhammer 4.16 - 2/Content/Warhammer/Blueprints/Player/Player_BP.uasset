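; Player character Blueprint that ties a custom PlayerMovementComponent to player input and nearby NPC detection.
; The construction script casts the character movement to that component and hands it a self reference, while BeginPlay caches the Player_Controller.
; Each tick passes NPCs overlapping OverlapCollider to the component's FilterEnemies and redundantly tells the capsule to ignore itself.
; RotateSpringArm input sets the RotateArm flag while held and calls ResetArm on release.
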(event `self.ReceiveBeginPlay`
  (bind _asplayer_controller (cast `Player_Controller` (`self.GetController`)))
  (set `self.playerController` _asplayer_controller))

(event `self.ReceiveTick`
  (params (DeltaSeconds :type "Float (single-precision)"))
  (bind _capsulecomponent (`self.CapsuleComponent`))
  (`PrimitiveComponent.IgnoreActorWhenMoving` _capsulecomponent self true)
  (`PrimitiveComponent.IgnoreActorWhenMoving` _capsulecomponent self true)
  (`PlayerMovementComponent.FilterEnemies` (`self.movementComponent`) (`PrimitiveComponent.GetOverlappingActors` (`self.Overlap Collider`) "/Script/Warhammer.NPC")))

(event `InputAction|RotateSpringArm`
  (params (Key :type "Key Structure" :default "AnyKey"))
  (:`Pressed`
    (set `self.RotateArm` true))
  (:`Released`
    (set `self.RotateArm` false)
    (`self.ResetArm`)))

(fn `UserConstructionScript`
  (bind _output_get (set `self.player` self))
  (bind _asplayer_movement_component (cast `PlayerMovementComponent` (`self.CharacterMovement`))
    (:`then`
      (bind _output_get_2 (set `self.movementComponent` _asplayer_movement_component))
      (set `PlayerMovementComponent.playerChar` _output_get _output_get_2))
    (:`CastFailed`
      (`KismetSystemLibrary.PrintString` "movment cast failed"))))