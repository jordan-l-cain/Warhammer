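; Greenskin NPC character Blueprint for a Warhammer game that tracks the actors around it and sets up references for its custom movement.
; The construction script stores a self reference and caches the character movement component as an NPCMovementComponent.
; Every tick, the overlap collider and capsule are set to ignore the NPC itself when moving, and the collider's overlapping actors are saved to a variable.
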(event `self.ReceiveTick`
  (params (DeltaSeconds :type "Float (single-precision)"))
  (bind _overlapcollider (`self.OverlapCollider`))
  (`PrimitiveComponent.IgnoreActorWhenMoving` _overlapcollider self true)
  (`PrimitiveComponent.IgnoreActorWhenMoving` (`self.CapsuleComponent`) self true)
  (set `self.OverlappingActors` (`PrimitiveComponent.GetOverlappingActors` _overlapcollider null)))

(fn `UserConstructionScript`
  (set `self.npc` self)
  (bind _asnpcmovement_component (cast `NPCMovementComponent` (`self.CharacterMovement`)))
  (set `self.movementComponent` _asnpcmovement_component))